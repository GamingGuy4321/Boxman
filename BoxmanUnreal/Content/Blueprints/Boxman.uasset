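; Boxman is an enemy AI character that patrols a looping array of path points and chases the player (Samuel) when PawnSensing spots him.
; Sight and patrol share one AIMoveTo branch on SeesPlayer, advancing waypoints on success or failure.
; Overlaps pause movement for timed states: peeking at cover when unaware, or hit and recovery from an active thrown drill.
; A FindNearestPath helper exists but is never called here.
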(event OnSeePawn(PawnSensing)
  (params (Pawn :type Pawn%20Object%20Reference))
  ;[1 1 1] Boxman sees Player, and chases
  (bind _assamuel (Utilities|Casting|CastToSamuel Pawn))
  (Variables|Default|SetSeesPlayer true)
  ;[1 1 1] Array path for Boxman
  (if (Variables|Default|GetSeesPlayer)
    (AI|AIMoveTo self "0, 0, 0" _assamuel 5.0 false
      (:then
        (Variables|Default|SetSeesPlayer false)))
    (else
      (AI|AIMoveTo self "0, 0, 0" (Utilities|Array|Get(acopy) (Variables|Default|GetPath) (Variables|Default|GetIndex)) 5.0 false
        (:OnSuccess
          _)
        (:OnFail
          _))
      (bind _result (Math|Integer|IncrementInt (Variables|Default|GetIndex))
        (:%20%20
          (if (> _result (Utilities|Array|LastIndex (Variables|Default|GetPath)))
            (Variables|Default|SetIndex 0))
          (CallFunction|Pathing))))))

(event Custom|Pathing
  ;[1 1 1] Array path for Boxman
  (if (Variables|Default|GetSeesPlayer)
    ;[1 1 1] Boxman sees Player, and chases
    (AI|AIMoveTo self "0, 0, 0" (stale OnSeePawn(PawnSensing) _assamuel) 5.0 false
      (:then
        (Variables|Default|SetSeesPlayer false)))
    (else
      (AI|AIMoveTo self "0, 0, 0" (Utilities|Array|Get(acopy) (Variables|Default|GetPath) (Variables|Default|GetIndex)) 5.0 false
        (:OnSuccess
          _)
        (:OnFail
          _))
      (bind _result (Math|Integer|IncrementInt (Variables|Default|GetIndex))
        (:%20%20
          (if (> _result (Utilities|Array|LastIndex (Variables|Default|GetPath)))
            (Variables|Default|SetIndex 0))
          (CallFunction|Pathing))))))

(event Collision|EventActorBeginOverlap
  (params (OtherActor :type Actor%20Object%20Reference))
  ;[1 1 1] If Boxman overkaps with Rack, and doesn't see player play look around coner animation
  (Utilities|Casting|CastToCover_block_Blueprint OtherActor
    (:then
      (if (not (Variables|Default|GetSeesPlayer))
        (Variables|Default|SetIs%20moving false)
        (Pawn|Components|CharacterMovement|SetMovementMode (Variables|Character|GetCharacterMovement) "MOVE_None" 0)
        (Transformation|SetActorRotation "0,90.000000,0.000000")
        (Variables|Default|SetLookCoverleft true)
        (Utilities|FlowControl|Delay 3.6)
        (Variables|Default|SetLookCoverleft false)
        (Pawn|Components|CharacterMovement|SetMovementMode (Variables|Character|GetCharacterMovement) "MOVE_Walking" 0)
        (Variables|Default|SetIs%20moving true)))
    (:CastFailed
      ;[1 1 1] On overlap with throwable weapon, play hit animation
      (bind _array_element (Utilities|Array|ForEachLoopwithBreak (Variables|/Script/Engine.Actor|GetTags OtherActor))
        (:LoopBody
          (if (Utilities|Name|Equal(Name) _array_element "Throwable") ; This is a weapon
            (bind _assm_electric_drill_01a_blueprint (Utilities|Casting|CastToSM_ElectricDrill_01a_Blueprint OtherActor))
            (if (Variables|/Game/Blueprints/SM_ElectricDrill_01a_Blueprint.SM_ElectricDrill_01a_Blueprint_C|GetisActive _assm_electric_drill_01a_blueprint) ; Weapon is active
              (Variables|Default|SetIs%20moving false)
              (Variables|Default|SetIsHit true)
              (Pawn|Components|CharacterMovement|SetMovementMode (Variables|Character|GetCharacterMovement) "MOVE_None" 0)
              (Utilities|FlowControl|Delay 3.3)
              (Variables|Default|SetIsHit false)
              (Variables|Default|SetIsRecovering true)
              (Utilities|FlowControl|Delay 7.6)
              (Variables|Default|SetIsRecovering false)
              (Pawn|Components|CharacterMovement|SetMovementMode (Variables|Character|GetCharacterMovement) "MOVE_Walking" 0)
              (Variables|Default|SetIs%20moving true))))))))

(event EventBeginPlay
  (Variables|Default|SetIs%20moving true)
  (CallFunction|Pathing))

(fn ConstructionScript)

(fn FindNearestPath
  (params (Location :type Vector) (Path :type Array%20of%20Target%20Point%20Object%20References))
  (bind _output_get (Variables|Default|SetPath Path))
  (for (_array_element _array_index) _output_get
    (Variables|Default|SetIndex _array_index)
    (if (< (Math|Vector|Distance(Vector) (Transformation|GetActorLocation _array_element) Location) (LocalVariables|GetLocateNearest%20Path))
      (LocalVariables|SetLocateNearest%20Path (Math|Vector|Distance(Vector) (Transformation|GetActorLocation _array_element) Location)))))