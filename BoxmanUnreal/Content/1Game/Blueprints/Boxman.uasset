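; Boxman is an AI enemy character that wanders to random reachable points until pawn sensing spots Samuel, then chases him.
; Overlapping a cover block before sighting the player stops it for a timed look-around; afterward, that overlap re-issues the chase.
; An active thrown drill stops it through timed hit and recovery phases.
; Boolean flags track these states, and SeesPlayer is never cleared.
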(event OnSeePawn(PawnSensing)
  (params (Pawn :type Pawn%20Object%20Reference))
  ;[1 1 1] Boxman sees Player, and chases
  (Variables|Default|SetSeesPlayer true)
  (bind _assamuel (Utilities|Casting|CastToSamuel Pawn))
  (AI|AIMoveTo self "0, 0, 0" _assamuel 5.0 false))

(event Collision|EventActorBeginOverlap
  (params (OtherActor :type Actor%20Object%20Reference))
  ;[1 1 1] If Boxman overkaps with Rack, and doesn't see player play look around coner animation
  (Utilities|Casting|CastToCover_block_Blueprint OtherActor
    (:then
      (if (Variables|Default|GetSeesPlayer)
        ;[1 1 1] Boxman sees Player, and chases
        (AI|AIMoveTo self "0, 0, 0" (stale OnSeePawn(PawnSensing) _assamuel) 5.0 false)
        (else
          (Variables|Default|SetIs%20moving false)
          (Pawn|Components|CharacterMovement|SetMovementMode (Variables|Character|GetCharacterMovement) "MOVE_None" 0)
          (Transformation|SetActorRotation "0,90.000000,0.000000")
          (Variables|Default|SetLookCoverleft true)
          (Utilities|FlowControl|Delay 3.6)
          (Variables|Default|SetLookCoverleft false)
          (Pawn|Components|CharacterMovement|SetMovementMode (Variables|Character|GetCharacterMovement) "MOVE_Walking" 0)
          (Variables|Default|SetIs%20moving true))))
    (:CastFailed
      ;[1 1 1] On overlap with throwable weapon, play hit animation
      (bind _array_element (Utilities|Array|ForEachLoopwithBreak (Variables|/Script/Engine.Actor|GetTags OtherActor))
        (:LoopBody
          (if (Utilities|Name|Equal(Name) _array_element "Throwable") ; This is a weapon
            (bind _assm_electric_drill_01a_blueprint (Utilities|Casting|CastToSM_ElectricDrill_01a_Blueprint OtherActor))
            (if (Variables|/Game/1Game/Blueprints/SM_ElectricDrill_01a_Blueprint.SM_ElectricDrill_01a_Blueprint_C|GetisActive _assm_electric_drill_01a_blueprint) ; Weapon is active
              (Variables|Default|SetIs%20moving false)
              (Variables|Default|SetIsHit true)
              (Pawn|Components|CharacterMovement|SetMovementMode (Variables|Character|GetCharacterMovement) "MOVE_None" 0)
              (Utilities|FlowControl|Delay 3.3)
              (Variables|Default|SetIsHit false)
              (Variables|Default|SetIsRecovering true)
              (Utilities|FlowControl|Delay 7.6)
              (Variables|Default|SetIsRecovering false)
              (Pawn|Components|CharacterMovement|SetMovementMode (Variables|Character|GetCharacterMovement) "MOVE_Walking" 0)
              (Variables|Default|SetIs%20moving true))))))))

(event EventTick
  (params (DeltaSeconds :type Float%20%28single-precision%29))
  ;[1 1 1] Array path for Boxman
  (if (not (Variables|Default|GetSeesPlayer))
    (if (not (Variables|Default|GetIs%20moving))
      (AI|AIMoveTo self (.RandomLocation (AI|Navigation|GetRandomReachablePointinRadius (Transformation|GetActorLocation) 2.5e+03 0 0)) 0 5.0 false
        (:then
          (Variables|Default|SetIs%20moving true))
        (:OnSuccess
          (Variables|Default|SetIs%20moving false :!label _label))
        (:OnFail
          (goto _label))))))

(fn ConstructionScript)